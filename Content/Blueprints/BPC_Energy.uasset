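; Actor component that tracks an energy pool for its owner, with death tied to running out of energy.
; CurrentEnergy starts at MaxEnergy on BeginPlay.
; DecreaseEnergy drains it with a floor of zero and sets IsDead from whether it is empty, while IncreaseEnergy refills it up to the maximum without updating IsDead.
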(event EventBeginPlay
  (Variables|Default|SetCurrentEnergy (Variables|Default|GetMaxEnergy)))

(event EventTick
  (params (DeltaSeconds :type Float%20%28single-precision%29)))

(fn DecreaseEnergy
  (params (EnergyDrain :type Float%20%28double-precision%29))
  (Variables|Default|SetCurrentEnergy (Math|Float|Max(Float) (- (Variables|Default|GetCurrentEnergy) EnergyDrain) 0.0))
  (Variables|Default|SetIsDead (<= (Variables|Default|GetCurrentEnergy) 0.0)))

(fn IncreaseEnergy
  (params (EnergyGain :type Float%20%28double-precision%29))
  (Variables|Default|SetCurrentEnergy (Math|Float|Min(Float) (+ EnergyGain (Variables|Default|GetCurrentEnergy)) (Variables|Default|GetMaxEnergy))))