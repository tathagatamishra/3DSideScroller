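; BP_Orbix is the player-controlled physics sphere, with energy and memory meters that drain over time.
; Enhanced Input moves it with acceleration forces and jumps it with an impulse, gated by death state and, for jumping, a hit-normal ground check.
; Looping timers drain both stats through BPCHealth, and loss and gain functions push values to the WBP_MainHUD bars it creates.
; Both HUD bars initialize from MaxEnergy, including memory.
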(event OnComponentHit(RedSphere)
  (params (HitComponent :type Primitive%20Component%20Object%20Reference) (OtherActor :type Actor%20Object%20Reference) (OtherComp :type Primitive%20Component%20Object%20Reference) (NormalImpulse :type Vector :default "0, 0, 0") (Hit :type Hit%20Result%20Structure%20%28by%20ref%29))
  ;[0.15 0.15 0.15 0.5] Jump if on ground using impulse
  (if (> (.z (.impactnormal Hit)) 0.6)
    (Variables|Default|SetIsGrounded true)))

(event Custom|EventApplyEnergyLoss
  ;[0.15 0.15 0.15 0.5] Player control
  (CallFunction|ApplyEnergyLoss 2.0))

(event Custom|EventApplyMemoryLoss
  ;[0.15 0.15 0.15 0.5] Player control
  (CallFunction|ApplyMemoryLoss 1.0))

(event Input|EnhancedActionEvents|EnhancedInputActionIA_Move
  (params (ActionValue :type Vector%202D%20Structure) (ElapsedSeconds :type Float%20%28double-precision%29) (TriggeredSeconds :type Float%20%28double-precision%29) (InputAction :type Input%20Action%20Object%20Reference :default "/Game/Input/IA_Move.IA_Move"))
  ;[0.15 0.15 0.15 0.5] Move using force
  (if (CallFunction|CanControl)
    (Physics|AddForce (Variables|Default|GetRedSphere) (* (Math|Vector|MakeVector (.y ActionValue) (.x ActionValue) 0.0) (Variables|Default|GetForceValue)) "None" true)))

(event Input|EnhancedActionEvents|EnhancedInputActionIA_Jump
  (params (ActionValue :type Boolean) (ElapsedSeconds :type Float%20%28double-precision%29) (TriggeredSeconds :type Float%20%28double-precision%29) (InputAction :type Input%20Action%20Object%20Reference :default "/Game/Input/IA_Jump.IA_Jump"))
  ;[0.15 0.15 0.15 0.5] Jump if on ground using impulse
  (if (and (Variables|Default|GetIsGrounded) (CallFunction|CanControl))
    (Physics|AddImpulse (Variables|Default|GetRedSphere) (Math|Vector|MakeVector 0.0 0.0 (Variables|Default|GetJumpForce)) "None" true)
    (Variables|Default|SetIsGrounded false)))

(event EventBeginPlay
  ;[0.15 0.15 0.15 0.5] Player control
  (Utilities|FlowControl|Sequence
    (:then_0
      (Input|AddMappingContext (PlayerController|LocalPlayerSubsystems|GetEnhancedInputLocalPlayerSubsystem (Game|GetPlayerController 0)) "/Game/Input/IMC_Default.IMC_Default" 0 "(bIgnoreAllPressedKeysUntilRelease=True,bForceImmediately=False,bNotifyUserSettings=False)"))
    (:then_1
      (bind _returnvalue (UserInterface|CreateWidget "/Game/Widgets/WBP_MainHUD.WBP_MainHUD_C"))
      (bind _output_get (Variables|Default|SetMainHUD _returnvalue))
      (UserInterface|Viewport|AddtoViewport _output_get 0)
      (Utilities|FlowControl|Sequence
        (:then_0
          (Default|InitEnergyBars (Variables|/Game/Widgets/WBP_MainHUD.WBP_MainHUD_C|GetWBP_EnergyBox (Variables|Default|GetMainHUD)) (Variables|/Game/Blueprints/BPC_Health.BPC_Health_C|GetMaxEnergy (Variables|Default|GetBPC_Health))))
        (:then_1
          (Default|InitMemoryBars (Variables|/Game/Widgets/WBP_MainHUD.WBP_MainHUD_C|GetWBP_MemoryBox (Variables|Default|GetMainHUD)) (Variables|/Game/Blueprints/BPC_Health.BPC_Health_C|GetMaxEnergy (Variables|Default|GetBPC_Health))))))
    (:then_2
      (Utilities|Time|SetTimerbyEvent (delegate Custom|EventApplyMemoryLoss) 5.0 true))
    (:then_3
      (Utilities|Time|SetTimerbyEvent (delegate Custom|EventApplyEnergyLoss) 5.0 true))))

(fn ConstructionScript)

(fn ApplyEnergyLoss
  (params (EnergyLoss :type Float%20%28double-precision%29))
  (Default|DecreaseEnergy (Variables|Default|GetBPC_Health) EnergyLoss)
  (Default|UpdateEnergyBar (Variables|/Game/Widgets/WBP_MainHUD.WBP_MainHUD_C|GetWBP_EnergyBox (Variables|Default|GetMainHUD)) (Variables|/Game/Blueprints/BPC_Health.BPC_Health_C|GetCurrentEnergy (Variables|Default|GetBPC_Health))))

(fn CanControl
  (return (not (Variables|/Game/Blueprints/BPC_Health.BPC_Health_C|GetIsDead (Variables|Default|GetBPC_Health)))))

(fn ApplyEnergyGain
  (params (EnergyGain :type Float%20%28double-precision%29))
  (Default|IncreaseEnergy (Variables|Default|GetBPC_Health) EnergyGain)
  (Default|UpdateEnergyBar (Variables|/Game/Widgets/WBP_MainHUD.WBP_MainHUD_C|GetWBP_EnergyBox (Variables|Default|GetMainHUD)) (Variables|/Game/Blueprints/BPC_Health.BPC_Health_C|GetCurrentEnergy (Variables|Default|GetBPC_Health))))

(fn ApplyMemoryGain
  (params (MemoryGain :type Float%20%28double-precision%29))
  (Default|RecoverMemory (Variables|Default|GetBPC_Health) MemoryGain)
  (Default|UpdateMemoryBar (Variables|/Game/Widgets/WBP_MainHUD.WBP_MainHUD_C|GetWBP_MemoryBox (Variables|Default|GetMainHUD)) (Variables|/Game/Blueprints/BPC_Health.BPC_Health_C|GetCurrentMemory (Variables|Default|GetBPC_Health))))

(fn ApplyMemoryLoss
  (params (MemoryLoss :type Float%20%28double-precision%29))
  (Default|CorruptMemory (Variables|Default|GetBPC_Health) MemoryLoss)
  (Default|UpdateMemoryBar (Variables|/Game/Widgets/WBP_MainHUD.WBP_MainHUD_C|GetWBP_MemoryBox (Variables|Default|GetMainHUD)) (Variables|/Game/Blueprints/BPC_Health.BPC_Health_C|GetCurrentMemory (Variables|Default|GetBPC_Health))))