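; BPC_Health is a component that tracks two depletable pools, Energy and Memory, for its owner.
; On BeginPlay both pools start at their maximum values.
; Functions decrease or restore each pool, clamped between zero and its maximum, and the decrease functions set IsDead when Energy empties and IsCorrupted when Memory empties.
; Restoring a pool does not clear its flag, and the component uses no Tick logic.
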(event EventBeginPlay
  (Variables|Default|SetCurrentEnergy (Variables|Default|GetMaxEnergy))
  (Variables|Default|SetCurrentMemory (Variables|Default|GetMaxMemory)))

(event EventTick
  (params (DeltaSeconds :type Float%20%28single-precision%29)))

(fn DecreaseEnergy
  (params (EnergyLoss :type Float%20%28double-precision%29))
  (Variables|Default|SetCurrentEnergy (Math|Float|Max(Float) (- (Variables|Default|GetCurrentEnergy) EnergyLoss) 0.0))
  (Variables|Default|SetIsDead (<= (Variables|Default|GetCurrentEnergy) 0.0)))

(fn IncreaseEnergy
  (params (EnergyGain :type Float%20%28double-precision%29))
  (Variables|Default|SetCurrentEnergy (Math|Float|Min(Float) (+ EnergyGain (Variables|Default|GetCurrentEnergy)) (Variables|Default|GetMaxEnergy))))

(fn RecoverMemory
  (params (MemoryGain :type Float%20%28double-precision%29))
  (Variables|Default|SetCurrentMemory (Math|Float|Min(Float) (+ MemoryGain (Variables|Default|GetCurrentMemory)) (Variables|Default|GetMaxMemory))))

(fn CorruptMemory
  (params (MemoryLoss :type Float%20%28double-precision%29))
  (Variables|Default|SetCurrentMemory (Math|Float|Max(Float) (- (Variables|Default|GetCurrentMemory) MemoryLoss) 0.0))
  (Variables|Default|SetIsCorrupted (<= (Variables|Default|GetCurrentMemory) 0.0)))