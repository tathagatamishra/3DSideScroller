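; Enemy drone AI that locks onto the first BP_Orbix pawn it sees through PawnSensing.
; Each Tick it moves toward the target while beyond AttackDistance, otherwise strafes sideways at half input, smoothly turning to face it with rotation lerps.
; A FlipFlop timer event is meant to switch strafe direction, but only its A branch is wired, so StrafeRight is only ever set false.
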(event OnSeePawn(PawnSensing)
  (params (Pawn :type Pawn%20Object%20Reference))
  (Variables|Default|GetTarget
    (:then)
    (:else
      (bind _asbp_orbix (Utilities|Casting|CastToBP_Orbix Pawn))
      (Variables|Default|SetTarget _asbp_orbix))))

(event Custom|ChangeStrafeDirection
  (Utilities|FlowControl|FlipFlop
    (:A
      (Variables|Default|SetStrafeRight false)
      (Utilities|Time|SetTimerbyEvent (delegate Custom|ChangeStrafeDirection) (Math|Random|RandomFloatinRange 2.0 3.0)))))

(event EventTick
  (params (DeltaSeconds :type Float%20%28single-precision%29))
  (bind _returnvalue (Transformation|GetActorLocation))
  (bind _target (Variables|Default|GetTarget)
    (:then
      (if (> (Transformation|GetDistanceTo _target) (Variables|Default|GetAttackDistance))
        (Pawn|Input|AddMovementInput (Math|Rotator|GetRotationXVector (Math|Rotator|MakeRotator 0.0 0.0 (.yaw (Math|Rotator|FindLookatRotation _returnvalue (+ (Transformation|GetActorLocation _target) "0.000000,0.000000,100.000000"))))) 1.0 false)
        (Transformation|SetActorRotation (Math|Rotator|Lerp(Rotator) (Transformation|GetActorRotation) (Math|Rotator|MakeRotator 0.0 0.0 (.yaw (Math|Rotator|FindLookatRotation _returnvalue (+ (Transformation|GetActorLocation _target) "0.000000,0.000000,100.000000")))) 0.1 true))
        (else
          (Pawn|Input|AddMovementInput (Math|Vector|GetRightVector (Math|Rotator|FindLookatRotation _returnvalue (Transformation|GetActorLocation _target))) (Math|Float|SelectFloat 0.5 -0.5 (Variables|Default|GetStrafeRight)) false)
          (Transformation|SetActorRotation (Math|Rotator|Lerp(Rotator) (Transformation|GetActorRotation) (Math|Rotator|FindLookatRotation _returnvalue (Transformation|GetActorLocation _target)) 0.1 true)))))
    (:else)))

(event EventBeginPlay
  (CallFunction|ChangeStrafeDirection))

(fn ConstructionScript)